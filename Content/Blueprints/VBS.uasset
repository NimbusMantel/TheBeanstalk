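; VBS is a Blueprint that randomizes the leaf look of its StalkPlants component when play begins.
; It creates a dynamic instance of M_Stalk_Leaves on the first material slot.
; It then sets six leaf scalar parameters to 0 or 1, each from its own random roll with a one-in-three chance of 1.
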(event EventBeginPlay
  (bind _returnvalue (Rendering|Material|CreateDynamicMaterialInstance (Variables|Default|GetStalkPlants) 0 "/Game/Materials/M_Stalk_Leaves.M_Stalk_Leaves" :!class /Script/Engine.PrimitiveComponent))
  (bind _output_get (Variables|Default|SetLeavesMaterial _returnvalue))
  (Rendering|Material|SetScalarParameterValue _output_get "Leaf01" (Math|Conversions|ToFloat(Boolean) (== (Math|Random|RandomIntegerinRange 1 3) 1)) :!class /Script/Engine.MaterialInstanceDynamic)
  (Rendering|Material|SetScalarParameterValue _output_get "Leaf02" (Math|Conversions|ToFloat(Boolean) (== (Math|Random|RandomIntegerinRange 1 3) 2)) :!class /Script/Engine.MaterialInstanceDynamic)
  (Rendering|Material|SetScalarParameterValue _output_get "Leaf03" (Math|Conversions|ToFloat(Boolean) (== (Math|Random|RandomIntegerinRange 1 3) 3)) :!class /Script/Engine.MaterialInstanceDynamic)
  (Rendering|Material|SetScalarParameterValue _output_get "Leaf04" (Math|Conversions|ToFloat(Boolean) (== (Math|Random|RandomIntegerinRange 1 3) 3)) :!class /Script/Engine.MaterialInstanceDynamic)
  (Rendering|Material|SetScalarParameterValue _output_get "Leaf05" (Math|Conversions|ToFloat(Boolean) (== (Math|Random|RandomIntegerinRange 1 3) 2)) :!class /Script/Engine.MaterialInstanceDynamic)
  (Rendering|Material|SetScalarParameterValue _output_get "Leaf06" (Math|Conversions|ToFloat(Boolean) (== (Math|Random|RandomIntegerinRange 1 3) 1)) :!class /Script/Engine.MaterialInstanceDynamic))

(fn ConstructionScript)