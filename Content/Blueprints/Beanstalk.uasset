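; Beanstalk segment actor for a climbing game, with three climbable knot rows and a death point marker for its height.
; SpawnKnots builds jittered StalkKnot child actors from a three-character pattern and applies the orientation-help setting; GetKnotVector returns each knot's position and rotation.
; GetAttachPoint supplies a transform with random yaw turn, limited by the Left/Right class name.
; The death widget fades in as the player nears vertically, or is destroyed if unused.
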(event EventBeginPlay
  ;[1 1 1] Initialize the death point display
  ;;[1 1 1] Cast to the death point widget
  (bind _asplayer_death_display (Utilities|Casting|CastToPlayerDeathDisplay (UserInterface|GetUserWidgetObject (Variables|Default|GetDeathPointDisplay))))
  (bind _success (Default|SetHeight _asplayer_death_display (Math|Float|Floor (/ (.Z (Math|Vector|BreakVector (Transformation|GetActorLocation))) 1e+02))))
  ;;[1 1 1] Destroy the death point widget if there's no death point
  (Variables|Default|SetDisplay _success)
  (if (not _success)
    (Components|DestroyComponent (Variables|Default|GetDeathPointDisplay))))

(event EventActorBeginOverlap
  (params (OtherActor :type Actor%20Object%20Reference)))

(event EventTick
  (params (DeltaSeconds :type Float%20%28single-precision%29))
  (bind _returnvalue (Game|GetPlayerCharacter 0))
  (bind _returnvalue_2 (Class|Actor|GetVerticalDistanceto _returnvalue))
  ;[1 1 1] Create the death point widget's fading effect
  ;;[1 1 1] Only execute if possible and near
  (if (and (Variables|Default|GetDisplay) (<= _returnvalue_2 3.5e+02))
    ;;[1 1 1] Set the alpha value of the death point widget
    (bind _asplayer_death_display (Utilities|Casting|CastToPlayerDeathDisplay (UserInterface|GetUserWidgetObject (Variables|Default|GetDeathPointDisplay))))
    (Default|SetAlpha _asplayer_death_display (- 1.0 (/ _returnvalue_2 3.5e+02)))))

(fn ConstructionScript)

(fn GetAttachPoint
  (bind _self self)
  (bind _attachpoint (Variables|Default|GetAttachPoint))
  (bind _returnvalue (Transformation|GetWorldTransform _attachpoint))
  (bind _returnvalue_2 (Utilities|GetClass _self))
  (bind _returnvalue_3 (Utilities|GetClassDisplayName _returnvalue_2))
  (bind (_location _rotation _scale) (Math|Transform|BreakTransform _returnvalue))
  (bind (_pitch _yaw _roll) (Class|KismetMathLibrary|BreakRot _rotation))
  ;[1 1 1] Get attach point
  (return (Math|Transform|MakeTransform _location (Class|KismetMathLibrary|MakeRot _pitch (+ _yaw (Utilities|Select :Index (Math|Random|RandomIntegerinRange (Math|Conversions|ToInteger(Boolean) (or (Utilities|Enum|Equal(Enum) _returnvalue_3 "BeanstalkLightRight") (Utilities|Enum|Equal(Enum) _returnvalue_3 "BeanstalkRight"))) (- 2 (Math|Conversions|ToInteger(Boolean) (or (Utilities|Enum|Equal(Enum) _returnvalue_3 "BeanstalkLeft") (Utilities|Enum|Equal(Enum) _returnvalue_3 "BeanstalkLightLeft"))))) :Option%200 -36.0 :Option%201 0.0 :Option%202 36.0)) _roll) _scale)))

(fn SpawnKnots
  (params (NewBeanstalk :type String))
  (bind _returnvalue (Utilities|String|GetCharacterArrayfromString NewBeanstalk))
  ;[1 1 1] Spawn knots
  ;;[1 1 1] Randomize the knots' transformations
  (bind (_leftknottransform _middleknottransform _rightknottransform) (CallFunction|RandomizeKnotTransform))
  ;;[1 1 1] Generate the left knot
  (switch name (Utilities|String|StringToName (Utilities|Array|Get(acopy) _returnvalue))
    (:Default
      (bind _returnvalue_2 (AddComponent|AddChildActorComponent false _leftknottransform))
      (Variables|Default|SetLeftKnotReference _returnvalue_2))
    (:O
      (bind _returnvalue_3 (AddComponent|AddChildActorComponent false _leftknottransform))
      (Variables|Default|SetLeftKnotReference _returnvalue_3))
    (:X
      (bind _returnvalue_4 (AddComponent|AddChildActorComponent false _leftknottransform))
      (Variables|Default|SetLeftKnotReference _returnvalue_4))
    (:Q
      (bind _returnvalue_5 (AddComponent|AddChildActorComponent false _leftknottransform))
      (Variables|Default|SetLeftKnotReference _returnvalue_5)))
  ;;[1 1 1] Generate the middle knot
  (switch name (Utilities|String|StringToName (Utilities|Array|Get(acopy) _returnvalue 1))
    (:Default
      (bind _returnvalue_6 (AddComponent|AddChildActorComponent false _middleknottransform))
      (Variables|Default|SetMiddleKnotReference _returnvalue_6))
    (:O
      (bind _returnvalue_7 (AddComponent|AddChildActorComponent false _middleknottransform))
      (Variables|Default|SetMiddleKnotReference _returnvalue_7))
    (:X
      (bind _returnvalue_8 (AddComponent|AddChildActorComponent false _middleknottransform))
      (Variables|Default|SetMiddleKnotReference _returnvalue_8))
    (:Q
      (bind _returnvalue_9 (AddComponent|AddChildActorComponent false _middleknottransform))
      (Variables|Default|SetMiddleKnotReference _returnvalue_9)))
  ;;[1 1 1] Generate the right knot
  (switch name (Utilities|String|StringToName (Utilities|Array|Get(acopy) _returnvalue 2))
    (:Default
      (bind _returnvalue_10 (AddComponent|AddChildActorComponent false _rightknottransform))
      (Variables|Default|SetRightKnotReference _returnvalue_10))
    (:O
      (bind _returnvalue_11 (AddComponent|AddChildActorComponent false _rightknottransform))
      (Variables|Default|SetRightKnotReference _returnvalue_11))
    (:X
      (bind _returnvalue_12 (AddComponent|AddChildActorComponent false _rightknottransform))
      (Variables|Default|SetRightKnotReference _returnvalue_12))
    (:Q
      (bind _returnvalue_13 (AddComponent|AddChildActorComponent false _rightknottransform))
      (Variables|Default|SetRightKnotReference _returnvalue_13)))
  ;;[1 1 1] Get the orientation help
  (bind _asuser_game_instance (Utilities|Casting|CastToUserGameInstance (Game|GetGameInstance)))
  (switch Utilities|FlowControl|Switch|SwitchonECheckBoxState (Variables|/Game/Blueprints/UserGameInstance.UserGameInstance_C|GetShowOrientationHelp _asuser_game_instance)
    (:Unchecked
      (LocalVariables|SetChecked false :!label _label))
    (:Checked
      (LocalVariables|SetChecked true))
    (:Undetermined
      (goto _label)))
  ;;[1 1 1] Cast to the left knot
  (bind _asstalk_knot (Utilities|Casting|CastToStalkKnot (Variables|/Script/Engine.ChildActorComponent|GetChildActor (Variables|Default|GetLeftKnotReference))))
  (Variables|/Game/Blueprints/StalkKnot.StalkKnot_C|SetRow _asstalk_knot -1)
  (Default|ToggleOrientationHelp _asstalk_knot (LocalVariables|GetChecked))
  ;;[1 1 1] Cast to the middle knot
  (bind _asstalk_knot_2 (Utilities|Casting|CastToStalkKnot (Variables|/Script/Engine.ChildActorComponent|GetChildActor (Variables|Default|GetMiddleKnotReference))))
  (Variables|/Game/Blueprints/StalkKnot.StalkKnot_C|SetRow _asstalk_knot_2 0)
  (Default|ToggleOrientationHelp _asstalk_knot_2 (LocalVariables|GetChecked))
  ;;[1 1 1] Cast to the right knot
  (bind _asstalk_knot_3 (Utilities|Casting|CastToStalkKnot (Variables|/Script/Engine.ChildActorComponent|GetChildActor (Variables|Default|GetRightKnotReference))))
  (Variables|/Game/Blueprints/StalkKnot.StalkKnot_C|SetRow _asstalk_knot_3 1)
  (Default|ToggleOrientationHelp _asstalk_knot_3 (LocalVariables|GetChecked)))

(fn RandomizeKnotTransform
  ;[1 1 1] Randomize knot transform
  ;;[1 1 1] Get the knots' relative transform
  (bind _returnvalue (Transformation|GetRelativeTransform (Variables|Default|GetKnotSpawnLeft)))
  (bind _returnvalue_2 (Transformation|GetRelativeTransform (Variables|Default|GetKnotSpawnMiddle)))
  (bind _returnvalue_3 (Transformation|GetRelativeTransform (Variables|Default|GetKnotSpawnRight)))
  ;;[1 1 1] Call the randomization functions
  (bind _uniquetransform (CallFunction|RandomizeTransform _returnvalue 36.0))
  (bind _uniquetransform_2 (CallFunction|RandomizeTransform _returnvalue_2 0.0))
  (bind _uniquetransform_3 (CallFunction|RandomizeTransform _returnvalue_3 -36.0))
  (return _uniquetransform _uniquetransform_2 _uniquetransform_3))

(fn RandomizeTransform
  (params (StandardTransform :type Transform) (ZROT :type Float%20%28single-precision%29 :default 0.0))
  (bind (_location _rotation _scale) (Math|Transform|BreakTransform StandardTransform))
  (bind _returnvalue (Math|Random|RandomFloatinRange -5.0 5.0))
  (bind _returnvalue_2 (Math|Float|Absolute(Float) ZROT))
  (bind (_x _y _z) (Math|Vector|BreakVector _location))
  ;[1 1 1] Randomize transform
  (return (Math|Transform|MakeTransform (Math|Vector|MakeVector (+ _x (* (Math|Trig|Sin(Degrees) _returnvalue_2) _returnvalue -1.0)) (+ _y (* (Math|Trig|Cos(Degrees) _returnvalue_2) _returnvalue (/ ZROT _returnvalue_2))) (+ _z (Math|Random|RandomFloatinRange -5.0 5.0))) _rotation _scale)))

(fn GetKnotVector
  (params (Position :type Integer :default 0))
  (bind _returnvalue (Transformation|GetActorRotation))
  (bind (_pitch _yaw _roll) (Class|KismetMathLibrary|BreakRot _returnvalue))
  ;[1 1 1] Get knot vector
  ;;[1 1 1] Brach the different rows
  (switch int Position
    (:Default
      _)
    (:0
      ;;[1 1 1] Set the buffer values
      (LocalVariables|SetKnotVectorBuffer (Transformation|GetWorldLocation (Variables|Default|GetLeftKnotReference)))
      (LocalVariables|SetKnotRotatorBuffer (Class|KismetMathLibrary|MakeRot _pitch (+ _yaw 36.0) _roll)))
    (:1
      (LocalVariables|SetKnotVectorBuffer (Transformation|GetWorldLocation (Variables|Default|GetMiddleKnotReference)))
      (LocalVariables|SetKnotRotatorBuffer _returnvalue))
    (:2
      (LocalVariables|SetKnotVectorBuffer (Transformation|GetWorldLocation (Variables|Default|GetRightKnotReference)))
      (LocalVariables|SetKnotRotatorBuffer (Class|KismetMathLibrary|MakeRot _pitch (- _yaw 36.0) _roll))))
  (return (LocalVariables|GetKnotVectorBuffer) (LocalVariables|GetKnotRotatorBuffer)))